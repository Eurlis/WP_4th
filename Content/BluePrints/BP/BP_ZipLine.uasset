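; BP_ZipLine is a zipline actor that builds its visible wire between two sphere endpoints.
; The Construction Script places Wire at their midpoint, rotates it by the look-at rotation plus a 90-degree pitch offset, and scales Z by their distance to fit a cylinder mesh.
; The Event Graph holds only disabled events and unconnected drafts of that logic, with no riding or runtime behavior.
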(event EventBeginPlay)

(event Collision|EventActorBeginOverlap
  (params (OtherActor :type Actor%20Object%20Reference)))

(event EventTick
  (params (DeltaSeconds :type Float%20%28single-precision%29)))

(fn ConstructionScript
  ;[0.15 0.15 0.15 0.5] 중점
  (Transformation|SetWorldLocation (Variables|Default|GetWire) (/ (+ (Transformation|GetWorldLocation (Variables|Default|GetSphere)) (Transformation|GetWorldLocation (Variables|Default|GetSphere1))) 2.0) false false)
  ;[0.15 0.15 0.15 0.5] 회전 계산
  (Transformation|SetWorldRotation (Variables|Default|GetWire) (Math|Rotator|CombineRotators (Math|Rotator|FindLookatRotation (Transformation|GetWorldLocation (Variables|Default|GetSphere)) (Transformation|GetWorldLocation (Variables|Default|GetSphere1))) (Math|Rotator|MakeRotator 0.0 9e+01 0.0)) false false)
  ;[0.15 0.15 0.15 0.5] 길이
  (Transformation|SetWorldScale3D (Variables|Default|GetWire) (Math|Vector|MakeVector 0.05 0.05 (/ (Math|Vector|VectorLength (- (Transformation|GetWorldLocation (Variables|Default|GetSphere)) (Transformation|GetWorldLocation (Variables|Default|GetSphere1)))) 1e+02))))