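; Base character Blueprint that shows a floating health and shield bar for an enemy passed to it.
; ShowEnemyHealth creates the bar widget if its validity check fails, stores the enemy, updates the values and restarts a short hide timer by function name.
; Tick projects a point above the tracked enemy to screen space and moves the widget there.
; The tracked enemy is not cleared when the bar hides.
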(event Custom|HideEnemyHealthBar
  (Widget|SetVisibility (Variables|Default|GetEnemyHealthBarWidget) "Hidden"))

(event EventBeginPlay)

(event Collision|EventActorBeginOverlap
  (params (OtherActor :type Actor%20Object%20Reference)))

(event EventTick
  (params (DeltaSeconds :type Float%20%28single-precision%29))
  (bind _trackedenemy (Variables|Default|GetTrackedEnemy))
  (bind _returnvalue (Transformation|GetActorLocation _trackedenemy))
  (Utilities|IsValid (Variables|Default|GetTrackedEnemy)
    (:Is%20Valid
      (Class|UserWidget|SetPositioninViewport (Variables|Default|GetEnemyHealthBarWidget) (.ScreenPosition (Class|GameplayStatics|ProjectWorldtoScreen (Game|GetPlayerController 0) (Math|Vector|MakeVector (.x _returnvalue) (.y _returnvalue) (+ (.z _returnvalue) 1.2e+02)) false)) true))))

(event EventShowEnemyHealth
  (params (EnemyActor :type Actor%20Object%20Reference) (HP :type Float%20%28single-precision%29) (MaxHp :type Float%20%28single-precision%29) (Shield :type Float%20%28single-precision%29) (MaxShield :type Float%20%28single-precision%29))
  (Utilities|IsValid "/Game/BluePrints/WBP/WBP_EnemyHealthBar.WBP_EnemyHealthBar"
    (:Is%20Valid
      _)
    (:Is%20Not%20Valid
      (bind _returnvalue (UserInterface|CreateWidget "/Game/BluePrints/WBP/WBP_EnemyHealthBar.WBP_EnemyHealthBar_C"))
      (bind _output_get (Variables|Default|SetEnemyHealthBarWidget _returnvalue))
      (UserInterface|Viewport|AddtoViewport _output_get 0)))
  (Variables|Default|SetTrackedEnemy EnemyActor)
  (Default|UpdateHealth (Variables|Default|GetEnemyHealthBarWidget) HP MaxHp Shield MaxShield)
  (Widget|SetVisibility (Variables|Default|GetEnemyHealthBarWidget) "Visible")
  (Utilities|Time|SetTimerbyFunctionName 0 "HideEnemyHealthBar" 3.0))

(fn ConstructionScript)